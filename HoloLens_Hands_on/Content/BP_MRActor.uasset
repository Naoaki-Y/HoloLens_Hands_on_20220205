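; Mixed reality test actor that starts an AR session with spatial mapping and exercises hand and gaze tracking.
; Each tick it draws debug spheres at every tracked hand keypoint and teleports its StaticMesh to a fixed distance along the gaze ray.
; The Spawn input creates a scaled-down BP_SpawnActor at the left hand's grip position with a limited life span.
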(event `self.ReceiveBeginPlay`
  (`ARBlueprintLibrary.ToggleARCapture` true "SpatialMapping")
  (`ARBlueprintLibrary.StartARSession` "/Game/DA_ARSessionConfig.DA_ARSessionConfig"))

(event `self.ReceiveTick`
  (params (DeltaSeconds :type "Float (single-precision)"))
  (`|ExecutionSequence`
    (:`then_0`
      (bind _enumvalue (foreach `EControllerHand` true)
        (:`LoopBody`
          (bind _motioncontrollerdata (`HeadMountedDisplayFunctionLibrary.GetMotionControllerData` null _enumvalue))
          (bind (_bvalid _devicename _applicationinstanceid _devicevisualtype _handindex _trackingstatus _gripposition _griprotation _aimposition _aimrotation _handkeypositions) (break `XRMotionControllerData` _motioncontrollerdata))
          (if (and _bvalid (`|EnumEquality` _devicevisualtype "Hand"))
            (bind _enumvalue_2 (foreach `EHandKeypoint` true)
              (:`LoopBody`
                (`KismetSystemLibrary.DrawDebugSphere` (`|GetArrayItem` _handkeypositions (`HandKeypointConversion.Conv_HandKeypointToInt32` _enumvalue_2)) 1.0 4)))))))
    (:`then_1`
      (bind _outgazedata (`EyeTrackerFunctionLibrary.GetGazeData`))
      (bind (_gazeorigin _gazedirection) (break `EyeTrackerGazeData` _outgazedata))
      (`SceneComponent.K2_SetWorldLocation` (`self.StaticMesh`) (+ _gazeorigin (* _gazedirection 150.0)) false true))))

(event `InputAction|Spawn`
  (params (Key :type "Key Structure"))
  (:`Pressed`
    (bind _motioncontrollerdata (`HeadMountedDisplayFunctionLibrary.GetMotionControllerData` null "Left"))
    (bind _returnvalue (`|SpawnActorFromClass` "/Game/BP_SpawnActor.BP_SpawnActor_C" (`KismetMathLibrary.MakeTransform` (`.GripPosition` (break `XRMotionControllerData` _motioncontrollerdata)) (struct) (0.3 0.3 0.3)) "Undefined" "OverrideRootScale" null null))
    (`self.SetLifeSpan` _returnvalue 60.0)))

(fn `UserConstructionScript`)